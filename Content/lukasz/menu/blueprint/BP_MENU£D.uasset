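; 3D menu actor that hosts a menu3d widget and moves the player's view between linked menu actors.
; On BeginPlay it binds to the widget's transition event and disables its own collision.
; The event's index picks a target from the Linkedmenus array, ignoring invalid indices.
; The transition moves collision from this actor to the target and sets it as the view target, so only the destination menu stays collidable.
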(event Custom|transition%20to
  (params (newmwnu :type BP%20MENU£%20D%20Object%20Reference))
  (Collision|SetActorEnableCollision false)
  (Collision|SetActorEnableCollision newmwnu true)
  (Game|Player|SetViewTargetwithBlend (Game|GetPlayerController 0) newmwnu 0.0 "VTBlend_EaseInOut" 2.0 false))

(event Custom|transizionetramenu
  (params (menuindex :type Integer))
  (if (Utilities|Array|IsValidIndex (Variables|Default|Getlinkedmenus) menuindex)
    (CallFunction|Transitionto (Utilities|Array|Get(acopy) (Variables|Default|Getlinkedmenus) menuindex))))

(event EventBeginPlay
  (bind _asmenu_3d (Utilities|Casting|CastTomenu3d (UserInterface|GetUserWidgetObject (Variables|Default|GetWidget))))
  (EventDispatchers|BindEventtoTransitiontolinkmap _asmenu_3d (delegate Custom|transizionetramenu))
  (Collision|SetActorEnableCollision false))

(fn ConstructionScript)