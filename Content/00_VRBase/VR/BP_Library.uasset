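; Blueprint library for the VR base with a function that configures headset tracking for seated or standing/roomscale play.
; SetHMDTrackingLevel enables the HMD, then sets the tracking origin to Eye for seated or Floor for standing.
; It sets the VR camera origin's relative height from the player start counter Z, adding a seated adjustment when seated.
; Each branch prints a colored debug message naming the chosen mode.
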(fn SetHMDTrackingLevel
  (params (IsSeated :type Boolean) (ZSeatedAdjusment :type Float%20%28single-precision%29) (PlayerSartCounterZ :type Float%20%28single-precision%29) (VRCameraOrigin :type Scene%20Component%20Object%20Reference%20%28by%20ref%29))
  (Class|HeadMountedDisplayFunctionLibrary|EnableHMD true)
  (if IsSeated
    ;[1 1 1] Seated
    (Class|HeadMountedDisplayFunctionLibrary|SetTrackingOrigin "Eye")
    (Transformation|SetRelativeLocation VRCameraOrigin (Math|Vector|MakeVector 0.0 0.0 (+ ZSeatedAdjusment PlayerSartCounterZ)) false false)
    (Development|PrintString 0 "Seated  Traking Level" true true "(R=0.000000,G=1.000000,B=0.208865,A=1.000000)")
    (else
      ;[1 1 1] Standing / Roomscale
      (Class|HeadMountedDisplayFunctionLibrary|SetTrackingOrigin "Floor")
      (Transformation|SetRelativeLocation VRCameraOrigin (Math|Vector|MakeVector 0.0 0.0 PlayerSartCounterZ) false false)
      (Development|PrintString 0 "Standing Traking Level" true true "(R=1.000000,G=0.016463,B=0.000000,A=1.000000)"))))